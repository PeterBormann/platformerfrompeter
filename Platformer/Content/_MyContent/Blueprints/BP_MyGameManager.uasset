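; Game manager Blueprint that tracks the game state (Running, Win, Lose, Abandon) and switches the matching end screens.
; Init creates the three end-screen widgets and sets Running.
; SetState hides the UI, then on a state change shows that state's widget and the mouse, or hides the mouse when Running.
; ResetGame moves the player to the first PlayerStart and re-runs Init, which creates new widgets each time.
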(event EventBeginPlay)

(event Collision|EventActorBeginOverlap
  (params (OtherActor :type Actor%20Object%20Reference)))

(event EventTick
  (params (DeltaSeconds :type Float%20%28single-precision%29)))

(fn ConstructionScript)

(fn Init
  (CallFunction|CreateUI)
  (CallFunction|SetState "NewEnumerator0"))

(fn SetState
  (params (NewState :type BP_MyGameStates%20Enum :default "NewEnumerator0"))
  (CallFunction|HideUI)
  (if (Utilities|Enum|NotEqual(Enum) NewState (Variables|Default|GetCurrentGameState))
    (bind _output_get (Variables|Default|SetCurrentGameState NewState))
    (switch Utilities|FlowControl|Switch|SwitchonBP_MyGameStates _output_get
      (:NewEnumerator0
        (CallFunction|ShowMouse false))
      (:NewEnumerator1
        (Widget|SetVisibility (Variables|Default|GetWidgetWin) "Visible")
        (CallFunction|ShowMouse true :!label _label))
      (:NewEnumerator2
        (Widget|SetVisibility (Variables|Default|GetWidgetLoose) "Visible")
        (goto _label))
      (:NewEnumerator3
        (Widget|SetVisibility (Variables|Default|GetWidgetAbandon) "Visible")
        (goto _label)))))

(fn GetState
  (return (Variables|Default|GetCurrentGameState)))

(fn CreateUI
  (bind _returnvalue (UserInterface|CreateWidget "/Game/_MyContent/UI/Widget_Abandon.Widget_Abandon_C"))
  (bind _output_get (Variables|Default|SetWidgetAbandon _returnvalue))
  (UserInterface|Viewport|AddtoViewport _output_get 0)
  (bind _returnvalue_2 (UserInterface|CreateWidget "/Game/_MyContent/UI/WidgetLoose.WidgetLoose_C"))
  (bind _output_get_2 (Variables|Default|SetWidgetLoose _returnvalue_2))
  (UserInterface|Viewport|AddtoViewport _output_get_2 0)
  (bind _returnvalue_3 (UserInterface|CreateWidget "/Game/_MyContent/UI/WidgetWin.WidgetWin_C"))
  (bind _output_get_3 (Variables|Default|SetWidgetWin _returnvalue_3))
  (UserInterface|Viewport|AddtoViewport _output_get_3 0))

(fn ResetGame
  (bind _outactors (Actor|GetAllActorsOfClass "/Script/Engine.PlayerStart"))
  (Transformation|SetActorLocation (Variables|Default|GetMyPlayer) (Transformation|GetActorLocation (Utilities|Array|Get(acopy) _outactors)) false false)
  (bind _mygamemanager (CallFunction|GetMyGameManager))
  (CallFunction|Init _mygamemanager))