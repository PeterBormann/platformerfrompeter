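; BP_MySplinePlatform is a moving platform actor that travels along a spline path.
; On BeginPlay it plays a timeline at a configurable rate, and each update maps the timeline's normalized value to a distance along the spline to set the mesh's world location without sweeping.
; The construction script applies the configurable static mesh and material to the platform mesh.
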(event Custom|PlatformStart
  (bind _spline (Variables|Default|GetSpline))
  (Components|Timeline|SetPlayRate (Variables|Default|GetMotionTimeline) (Variables|Default|GetRate))
  (bind _splinedistance (Timeline|MotionTimeline Play)
    (:Update
      (Transformation|SetWorldLocation (Variables|Default|GetPlatformMesh) (Spline|GetLocationatDistanceAlongSpline _spline (* _splinedistance (Spline|GetSplineLength _spline)) "World") false false))))

(event EventBeginPlay
  (CallFunction|PlatformStart))

(event Collision|EventActorBeginOverlap
  (params (OtherActor :type Actor%20Object%20Reference)))

(event EventTick
  (params (DeltaSeconds :type Float%20%28single-precision%29)))

(fn ConstructionScript
  (Components|StaticMesh|SetStaticMesh (Variables|Default|GetPlatformMesh) (Variables|Default|GetStaticMesh))
  (Rendering|Material|SetMaterial (Variables|Default|GetPlatformMesh) 0 (Variables|Default|GetMaterial)))