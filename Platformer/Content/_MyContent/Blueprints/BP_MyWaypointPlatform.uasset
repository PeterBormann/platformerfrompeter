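; Moving platform actor that travels through an array of waypoint actors, with configurable mesh, material, rate and optional looping.
; BeginPlay hides the waypoints and calls PlatformStart inside that loop, setting the first segment and playing MotionTimeline.
; The timeline lerps location between the current waypoint pair; its event advances the indices, or restarts from the first waypoint when looping.
; Start and Stop functions control the motion.
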(event Custom|PlatformStart
  (bind _motiontimeline (Variables|Default|GetMotionTimeline))
  (CallFunction|SetFirstWaypoint)
  (Components|Timeline|SetPlayRate _motiontimeline (Variables|Default|GetRate))
  (Components|Timeline|PlayfromStart _motiontimeline))

(event EventBeginPlay
  (for _array_element (Variables|Default|GetWaypoints)
    (Rendering|SetActorHiddenInGame _array_element true)
    (CallFunction|PlatformStart)))

(event Collision|EventActorBeginOverlap
  (params (OtherActor :type Actor%20Object%20Reference)))

(event EventTick
  (params (DeltaSeconds :type Float%20%28single-precision%29)))

(fn ConstructionScript
  (Components|StaticMesh|SetStaticMesh (Variables|Default|GetPlatformMesh) (Variables|Default|GetStaticMesh%20))
  (Rendering|Material|SetMaterial (Variables|Default|GetPlatformMesh) 0 (Variables|Default|GetMaterial)))

(fn SetPossitions
  (bind _waypoints (Variables|Default|GetWaypoints))
  (Variables|Default|SetCurrentWaypointPossition (Transformation|GetActorLocation (Utilities|Array|Get(acopy) _waypoints (Variables|Default|GetCurrentWaypoint%20Index))))
  (Variables|Default|SetNextWaypointPossition (Transformation|GetActorLocation (Utilities|Array|Get(acopy) _waypoints (Variables|Default|GetNextWaypoint%20Index)))))

(fn SetFirstWaypoint
  (Variables|Default|SetCurrentWaypoint%20Index 0)
  (Variables|Default|SetNextWaypoint%20Index 1)
  (CallFunction|SetPossitions))

(fn SetNextWaypoint
  (bind _result (Math|Integer|IncrementInt (Variables|Default|GetCurrentWaypoint%20Index))
    (:%20%20
      (Variables|Default|SetNextWaypoint%20Index (+ _result 1))
      (CallFunction|SetPossitions))))

(fn PathIsFinished
  (return (== (Variables|Default|GetNextWaypoint%20Index) (- (Utilities|Array|Length (Variables|Default|GetWaypoints)) 1))))

(fn Start
  (CallFunction|PlatformStart))

(fn Stop
  (Audio|Components|Audio|Stop (Variables|Default|GetMotionTimeline)))